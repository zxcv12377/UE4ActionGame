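; HP potion item that spins and sparkles in the world and restores a fixed amount of the player's health when used.
; Interact reads a hardcoded ItemDataTable row, adds it to the player's inventory widget, plays a pickup effect and destroys the actor.
; UseItem heals the player character, clamped to MaxHP.
; Tick drives the spin by adding DeltaSeconds to a constant step, so its speed depends on frame rate.
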(event `self.ReceiveActorBeginOverlap`
  (params (OtherActor :type "Actor Object Reference")))

(event `/Game/ActionGame/InteractBP.Interact`
  (bind _asplayer_character_bp (cast `/Game/ActionGame/PlayerCharacterBP` (`GameplayStatics.GetPlayerCharacter` 0)))
  (bind _returnvalue (`|GetDataTableRow` "/Game/ActionGame/ItemDataTable.ItemDataTable" "1")
    (:`then`
      (bind (_name _texture _type _equiptype _itemclass _description _count) (break `/Game/ActionGame/ItemDataBase` _returnvalue))
      (bind _output_get (set `self.itemInfo` (make `itemData` _name _texture _type _equiptype _itemclass _description _count)))
      (`/Game/ActionGame/Interface/InventoryWidgetBP.AddToInventory` (`/Game/ActionGame/PlayerCharacterBP.InventoryUMG` _asplayer_character_bp) _output_get)
      (`GameplayStatics.SpawnEmitterAttached` "/Game/InfinityBladeEffects/Effects/FX_Treasure/Gold_Bag/P_GoldSparkle_Bag_Pickup.P_GoldSparkle_Bag_Pickup" (`self.Root`))
      (`self.K2_DestroyActor`))))

(event `self.ReceiveBeginPlay`
  (`GameplayStatics.SpawnEmitterAttached` "/Game/InfinityBladeEffects/Effects/FX_Treasure/Gold_Bag/P_GoldSparkle_Bag_Loop.P_GoldSparkle_Bag_Loop" (`self.Root`) "None" (0.0 0.0 0.0) (struct) (1.0 1.0 1.0) "KeepRelativeOffset" false))

(event `/Game/ActionGame/InteractBP.UseItem`
  (bind _asplayer_character_bp (cast `/Game/ActionGame/PlayerCharacterBP` (`GameplayStatics.GetPlayerCharacter` 0)))
  (bind _returnvalue (+ (`PlayerCharacter.currentHP` _asplayer_character_bp) 50.0))
  (bind _maxhp (`PlayerCharacter.maxHP` _asplayer_character_bp))
  (if (> _returnvalue _maxhp)
    (set `PlayerCharacter.currentHP` _maxhp _asplayer_character_bp)
    (else
      (set `PlayerCharacter.currentHP` _returnvalue _asplayer_character_bp))))

(event `self.ReceiveTick`
  (params (DeltaSeconds :type "Float (single-precision)"))
  (`SceneComponent.K2_AddLocalRotation` (`self.Root`) (`KismetMathLibrary.MakeRotator` 0.0 0.0 (+ DeltaSeconds 1.0)) false false))

(fn `UserConstructionScript`)