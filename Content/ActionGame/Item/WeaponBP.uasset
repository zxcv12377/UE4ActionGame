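; WeaponBP is a weapon pickup that spins in the world and goes into the player's inventory on interaction.
; Interact reads the hard-coded row "3" of ItemDataTable, passes it as item info to the PlayerCharacterBP's InventoryUMG, then destroys the actor.
; Tick yaws the root by DeltaSeconds plus one degree each frame, so spin speed depends on frame rate.
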(event `/Game/ActionGame/InteractBP.Interact`
  ;[1 1 1] 아이템 정보를 인벤토리에 저장
  (bind _asplayer_character_bp (cast `/Game/ActionGame/PlayerCharacterBP` (`GameplayStatics.GetPlayerCharacter` 0)))
  (bind _returnvalue (`|GetDataTableRow` "/Game/ActionGame/ItemDataTable.ItemDataTable" "3")
    (:`then`
      (bind _output_get (set `self.itemInfo` (make `itemData` (break `/Game/ActionGame/ItemDataBase` _returnvalue) (`.texture_9_9A0102274624681F424383A70A057C85` (break `/Game/ActionGame/ItemDataBase` _returnvalue)) (`.Type_18_5823D4C44DB86FA390B33188B6EF43BA` (break `/Game/ActionGame/ItemDataBase` _returnvalue)) (`.EquipType_22_88935E6540DB69736BF3ACAA2FDC1298` (break `/Game/ActionGame/ItemDataBase` _returnvalue)) (`.ItemClass_19_969AFB7D4B6C633CF9935B9A3ECD2839` (break `/Game/ActionGame/ItemDataBase` _returnvalue)) (`.Description_15_89F891D14A0E6702141A04879D2C8E4B` (break `/Game/ActionGame/ItemDataBase` _returnvalue)) (`.Count_14_5869A44644C7E845DBB3778EEB0927D1` (break `/Game/ActionGame/ItemDataBase` _returnvalue)))))
      (`/Game/ActionGame/Interface/InventoryWidgetBP.AddToInventory` (`/Game/ActionGame/PlayerCharacterBP.InventoryUMG` _asplayer_character_bp) _output_get)
      (`self.K2_DestroyActor`))))

(event `self.ReceiveTick`
  (params (DeltaSeconds :type "Float (single-precision)"))
  ;[1 1 1] 아이템 회전
  (`SceneComponent.K2_AddLocalRotation` (`self.Root`) (`KismetMathLibrary.MakeRotator` 0.0 0.0 (+ DeltaSeconds 1.0)) false false))

(fn `UserConstructionScript`)