(event `self.ReceiveBeginPlay`
  (bind _defaultweapon (`self.DefaultWeapon`))
  ;[1 1 1] 게임 시작시 생성됨
  (bind _returnvalue (`|CreateWidget` "/Game/ActionGame/Interface/InventoryWidgetBP.InventoryWidgetBP_C"))
  (bind _output_get (set `self.InventoryUMG` _returnvalue))
  (`UserWidget.AddToViewport` _output_get 0)
  (bind _returnvalue_2 (`|CreateWidget` "/Game/ActionGame/Interface/EquipWidgetBP.EquipWidgetBP_C"))
  (bind _output_get_2 (set `self.EquipUMG` _returnvalue_2))
  (`/Game/ActionGame/Interface/InventoryWidgetBP.AddToInventory(MapChange)` _output_get)
  (`Widget.RemoveFromParent` _output_get)
  (`Widget.RemoveFromParent` _output_get_2)
  (set `self.actorLocation` (`GameplayStatics.GetPlayerCharacter` 0))
  (bind _returnvalue_3 (`|GetDataTableRow` "/Game/ActionGame/ItemDataTable.ItemDataTable" "4")
    (:`then`
      (bind (_name _texture _type _equiptype _itemclass _description _count) (break `/Game/ActionGame/ItemDataBase` _returnvalue_3))
      (set `self.BaseWaepon` (make `itemData` _name _texture _type _equiptype _itemclass _description _count))
      (`/Game/ActionGame/Interface/EquipWidgetBP.Weapon` _output_get_2 (`self.BaseWaepon`) true)
      (`KismetArrayLibrary.Array_Clear` _defaultweapon)
      (bind _returnvalue_4 (`|SpawnActorFromClass` _itemclass (`KismetMathLibrary.Conv_VectorToTransform` (`SceneComponent.GetSocketLocation` (`self.righthand`) "None")) "Undefined" "OverrideRootScale" null null))
      (bind _asweapon_actor (cast `WeaponActor` _returnvalue_4))
      (`KismetArrayLibrary.Array_Add` _defaultweapon (`WeaponActor.WeaponClass` _asweapon_actor))
      (`KismetArrayLibrary.Array_AddUnique` (`self.Inventory`) _asweapon_actor)
      (`self.WeaponAttach` _asweapon_actor)
      (set `self.MyWeapon` _returnvalue_4))))

(event `CheckSpeed`
  (bind (_returnvalue_x _returnvalue_y _returnvalue_z) (`KismetMathLibrary.BreakVector` (`self.GetVelocity`)))
  ;[1 1 1] 높은곳 낙하
  (if (`|EnumEquality` (stale `self.K2_OnMovementModeChanged` NewMovementMode) "MOVE_Falling") :!label _label
    (if (<= _returnvalue_z -1500.0)
      (set `self.isHardLanging` true)
      (set `self.isJump` true)
      (else
        (`KismetSystemLibrary.Delay` 0.2)
        (`self.CheckSpeed`)))))

(event `self.K2_OnMovementModeChanged`
  (params (PrevMovementMode :type "EMovementMode Enum" :default "MOVE_None") (NewMovementMode :type "EMovementMode Enum" :default "MOVE_None") (PrevCustomMode :type Byte) (NewCustomMode :type Byte))
  (bind _charactermovement (`self.CharacterMovement`))
  ;[1 1 1] 높은곳 낙하
  (`|ExecutionSequence`
    (:`then_0`
      (goto _label))
    (:`then_1`
      (if (and (`|EnumEquality` NewMovementMode "MOVE_Walking") (`self.isHardLanging`))
        (`CharacterMovementComponent.DisableMovement` _charactermovement)
        (bind _returnvalue (`self.PlayAnimMontage` "/Game/ActionGame/Player/Animation/Player_Falling_To_Landing_Montage.Player_Falling_To_Landing_Montage"))
        (set `self.isHardLanging` false)
        (set `self.isJump` false)
        (`KismetSystemLibrary.Delay` _returnvalue)
        (`CharacterMovementComponent.SetMovementMode` _charactermovement "MOVE_Walking" 0)))))

(event `WeaponAttach`
  (params (Weapon :type "Actor Object Reference"))
  ;[1 1 1] 무기 장착시 손에 붙이기
  (bind _asweapon_actor (cast `WeaponActor` Weapon))
  (`SceneComponent.K2_AttachToComponent` (`WeaponActor.Handle` _asweapon_actor) (`self.Mesh`) "RightHand" "KeepRelative" "KeepRelative" "KeepRelative" true))

(event `Key|F`
  (params (Key :type "Key Structure"))
  ;[1 1 1] 아이템 상호작용
  (:`Pressed`
    (for _array_element (`self.GetOverlappingActors` "/Script/Engine.Actor")
      (if (`KismetSystemLibrary.DoesImplementInterface` _array_element "/Game/ActionGame/InteractBP.InteractBP_C")
        (message `/Game/ActionGame/InteractBP.Interact` _array_element)
        (break)))))

(event `levelupParticlePlay`
  ;[1 1 1] 레벨업 FX
  (`GameplayStatics.SpawnEmitterAttached` "/Game/ActionGame/P_levelUp.P_levelUp" (`self.BasicLocationZ0`)))

(event `Key|I`
  (params (Key :type "Key Structure"))
  (bind _returnvalue (`GameplayStatics.GetPlayerController` 0))
  (bind _inventoryumg (`self.InventoryUMG`))
  ;[1 1 1] 인벤토리
  (:`Pressed`
    (`/Engine/EditorBlueprintResources/StandardMacros.FlipFlop`
      (:`A`
        (`UserWidget.AddToViewport` _inventoryumg 0)
        (set `PlayerController.bShowMouseCursor` true _returnvalue)
        (`WidgetBlueprintLibrary.SetInputMode_GameAndUIEx` _returnvalue (`self.InventoryUMG`)))
      (:`B`
        (`Widget.RemoveFromParent` _inventoryumg)
        (set `PlayerController.bShowMouseCursor` false _returnvalue)
        (`WidgetBlueprintLibrary.SetInputMode_GameOnly` _returnvalue)))))

(event `Key|E`
  (params (Key :type "Key Structure"))
  (bind _returnvalue (`GameplayStatics.GetPlayerController` 0))
  (bind _equipumg (`self.EquipUMG`))
  ;[1 1 1] 장비창
  (:`Pressed`
    (`/Engine/EditorBlueprintResources/StandardMacros.FlipFlop`
      (:`A`
        (`UserWidget.AddToViewport` _equipumg 0)
        (set `PlayerController.bShowMouseCursor` true _returnvalue)
        (`WidgetBlueprintLibrary.SetInputMode_GameAndUIEx` _returnvalue (`self.InventoryUMG`)))
      (:`B`
        (`Widget.RemoveFromParent` _equipumg)
        (set `PlayerController.bShowMouseCursor` false _returnvalue)
        (`WidgetBlueprintLibrary.SetInputMode_GameOnly` _returnvalue)))))

(event `Key|RightMouseButton`
  (params (Key :type "Key Structure"))
  ;[1 1 1] 무기 스킬 발동
  (:`Pressed`
    (set `self.isDot` true)
    (`/Engine/EditorBlueprintResources/StandardMacros.IsValid` (`self.WeaponGetSkillParticle`)
      (:`Is Valid`
        (if (>= (`self.currentMP`) (`self.WeaponMPAmount`))
          (if (`self.isAttack`)
            _
            (elif (`self.isRolling`)
              _
              (elif (`self.isJump`)
                _
                (elif (`self.isSkill`)
                  _
                  (elif (not (`self.isMouseCursor`))
                    (set `self.isSkill` true)
                    (switch `int` (`self.AttackType_0`) ; 0번은 플레이어 밑에 생성\n1번은 플레이어에 붙임
                      (:`0`
                        (`GameplayStatics.SpawnEmitterAtLocation` (`self.WeaponGetSkillParticle`) (`self.EmitterLocation_0`) (struct) (1.0 1.0 1.0) true "AutoRelease"))
                      (:`1`
                        _))
                    (set `self.currentMP` (- (`self.currentMP`) (`self.WeaponMPAmount`)))
                    (switch `int` (`self.RadialOrNormalOrDot`) ; 0번은 범위 공격\n1번은 단일 공격\n2번은 도트 공격
                      (:`0`
                        ;;[1 1 1] 범위 타입
                        (set `self.isSkill` false)
                        (`GameplayStatics.ApplyRadialDamage` (`self.BaseDamage_0`) (`self.K2_GetActorLocation` (`self.actorLocation`)) (`self.DamageRadius_0`) null (`self.ignore`) self null true))
                      (:`2`
                        ;;[1 1 1] 도트 타입
                        (`self.PlayAnimMontage` "/Game/ActionGame/Player/Animation/whirlwind.whirlwind" 1.5)
                        (bind _returnvalue (`GameplayStatics.SpawnEmitterAttached` (`self.WeaponGetSkillParticle`) (`self.BasicLocationMiddle`)))
                        (if (and (`self.isDot`) (>= (`self.currentMP`) (`self.WeaponMPAmount`))) :!label _label_2
                          (`GameplayStatics.ApplyRadialDamage` (`self.BaseDamage_0`) (`self.K2_GetActorLocation` (`self.actorLocation`)) (`self.DamageRadius_0`) null (`self.ignore`) self null true)
                          (`KismetSystemLibrary.Delay` 0.8)
                          (set `self.currentMP` (- (`self.currentMP`) (`self.WeaponMPAmount`)))
                          (goto _label_2)
                          (else
                            (`ActorComponent.K2_DestroyComponent` _returnvalue)
                            (`self.StopAnimMontage` "/Game/ActionGame/Player/Animation/whirlwind.whirlwind")
                            (set `self.isSkill` false))))))))))))))
  (:`Released`
    (set `self.isDot` false)))

(fn `UserConstructionScript`)